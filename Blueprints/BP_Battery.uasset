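; BP_Battery is a timed pickup that raises the player character's Health.
; On BeginPlay, a one-second Delay loop counts LifeSpan down and destroys the actor once it runs out.
; When a ThirdPersonCharacter overlaps Box_battery, it adds a point to that character's Health and the battery destroys itself.
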(event OnComponentBeginOverlap(Box_battery)
  (params (OverlappedComponent :type Primitive%20Component%20Object%20Reference) (OtherActor :type Actor%20Object%20Reference) (OtherComp :type Primitive%20Component%20Object%20Reference) (OtherBodyIndex :type Integer) (bFromSweep :type Boolean) (SweepResult :type Hit%20Result%20Structure%20%28by%20ref%29))
  (bind _asthird_person_character (Utilities|Casting|CastToThirdPersonCharacter OtherActor))
  (Variables|/Game/ThirdPersonBP/Blueprints/ThirdPersonCharacter.ThirdPersonCharacter_C|SetHealth _asthird_person_character (+ (Variables|/Game/ThirdPersonBP/Blueprints/ThirdPersonCharacter.ThirdPersonCharacter_C|GetHealth _asthird_person_character) 1.0))
  (Actor|DestroyActor))

(event EventBeginPlay
  (bind _output_get (Variables|Default|SetLife_span (- (Variables|Default|GetLife_span) 1.0) :!label _label))
  (if (<= _output_get 0.0)
    (Actor|DestroyActor)
    (else
      (Utilities|FlowControl|Delay 1.0)
      (goto _label))))

(event Collision|EventActorBeginOverlap
  (params (OtherActor :type Actor%20Object%20Reference)))

(event EventTick
  (params (DeltaSeconds :type Float%20%28single-precision%29)))

(fn ConstructionScript)