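; Spawner actor that continually drops BP_Battery and BP_Bomb actors at random positions in the level.
; BeginPlay spawns a battery, then loops on a one-second delay, spawning either a battery or a bomb by coin flip.
; Each spawn gets random X/Y in a square around the world origin, at the spawner's height.
; An unused-here Spawns function teleports the spawner to a random TargetPoint, with an index range that can overrun the array.
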(event EventBeginPlay
  (Game|SpawnActorfromClass "/Game/Blueprints/BP_Battery.BP_Battery_C" (Math|Conversions|ToTransform(Vector) (Math|Vector|MakeVector (Math|Random|RandomFloatinRange -1e+03 1e+03) (Math|Random|RandomFloatinRange -1e+03 1e+03) (.Z (Math|Vector|BreakVector (Transformation|GetActorLocation))))) "Undefined" 0 0 :!label _label)
  (Utilities|FlowControl|Delay 1.0 :!label _label_2)
  (if (Math|Random|RandomBool)
    (goto _label)
    (else
      (Game|SpawnActorfromClass "/Game/Blueprints/BP_Bomb.BP_Bomb_C" (Math|Conversions|ToTransform(Vector) (Math|Vector|MakeVector (Math|Random|RandomFloatinRange -1e+03 1e+03) (Math|Random|RandomFloatinRange -1e+03 1e+03) (.Z (Math|Vector|BreakVector (Transformation|GetActorLocation))))) "Undefined" 0 0)
      (goto _label_2))))

(event Collision|EventActorBeginOverlap
  (params (OtherActor :type Actor%20Object%20Reference)))

(event EventTick
  (params (DeltaSeconds :type Float%20%28single-precision%29)))

(fn ConstructionScript)

(fn Spawns
  (bind _outactors (Actor|GetAllActorsOfClass "/Script/Engine.TargetPoint"))
  (Transformation|Teleport (Transformation|GetActorLocation (Utilities|Array|Get(acopy) _outactors (Math|Random|RandomIntegerinRange 0 (Utilities|Array|Length _outactors)))) "0, 0, 0"))